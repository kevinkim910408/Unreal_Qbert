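; Enemy spawner that spawns red, green and purple ball actors during play.
; BeginPlay starts a randomized timer for red and green and an effectively fixed delay for purple.
; Red and green spawns re-arm their timers, while purple spawns once because its repeat timer is disconnected.
; Each ball spawns above a tile randomly picked from indices 1–2 of BP_MyMode's tile array and receives a CurrentTile.
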(event `SpawnRedBall`
  (bind _output (`|GetArrayItem` (`/Game/bp/BP_MyMode.Array of Tiles` (cast `/Game/bp/BP_MyMode` (`GameplayStatics.GetGameMode`) :!pure true)) (`KismetMathLibrary.RandomIntegerInRange` 1 2)))
  ;[1 1 1] Spawn Red Ball
  (`|SpawnActorFromClass` "/Game/bp/Enemy/BP_REDBALL.BP_REDBALL_C" (`KismetMathLibrary.MakeTransform` (+ (`self.K2_GetActorLocation` _output) (0.0 0.2 150.0))) "Undefined" "OverrideRootScale" null _output null)
  (`KismetSystemLibrary.K2_SetTimer` null "SpawnRedBall" (`KismetMathLibrary.RandomFloatInRange` 9.0 10.0)))

(event `SpawnGreenBall`
  (bind _output (`|GetArrayItem` (`/Game/bp/BP_MyMode.Array of Tiles` (cast `/Game/bp/BP_MyMode` (`GameplayStatics.GetGameMode`) :!pure true)) (`KismetMathLibrary.RandomIntegerInRange` 1 2)))
  ;[1 1 1] Spawn Green Ball
  (`|SpawnActorFromClass` "/Game/bp/Enemy/BP_GreenBall.BP_GreenBall_C" (`KismetMathLibrary.MakeTransform` (+ (`self.K2_GetActorLocation` _output) (0.0 0.2 150.0))) "Undefined" "OverrideRootScale" null _output null)
  (`KismetSystemLibrary.K2_SetTimer` null "SpawnGreenBall" (`KismetMathLibrary.RandomFloatInRange` 12.0 14.0)))

(event `SpawnPurpleBall`
  (bind _output (`|GetArrayItem` (`/Game/bp/BP_MyMode.Array of Tiles` (cast `/Game/bp/BP_MyMode` (`GameplayStatics.GetGameMode`) :!pure true)) (`KismetMathLibrary.RandomIntegerInRange` 1 2)))
  ;[1 1 1] Spawn Purple Ball
  (`|SpawnActorFromClass` "/Game/bp/Enemy/BP_PurpleBall.BP_PurpleBall_C" (`KismetMathLibrary.MakeTransform` (+ (`self.K2_GetActorLocation` _output) (0.0 0.2 150.0))) "Undefined" "OverrideRootScale" null _output null))

(event `self.ReceiveBeginPlay`
  ;[1 1 1] Begin Play
  ;[1 1 1] Actual Spawning
  ;;[1 1 1] Red Ball
  (`KismetSystemLibrary.K2_SetTimer` null "SpawnRedBall" (`KismetMathLibrary.RandomFloatInRange` 4.0 6.0))
  ;;[1 1 1] Green Ball
  (`KismetSystemLibrary.K2_SetTimer` null "SpawnGreenBall" (`KismetMathLibrary.RandomFloatInRange` 7.0 8.0))
  ;;[1 1 1] Purple Ball
  (`KismetSystemLibrary.K2_SetTimer` null "SpawnPurpleBall" (`KismetMathLibrary.RandomFloatInRange` 12.0 12.0)))

(fn `UserConstructionScript`)