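; BP_ENEMY is an enemy actor that drops onto a tile on spawn and can later fall off along an arc.
; BeginPlay spawns a BP_Spline, bends it over CurrentTile, and a timeline moves the enemy along it, then sets Activate to enable movement.
; FallAlongSpline reshapes the same spline over and below FailTileLocation, follows it with a second timeline, then destroys both spline and enemy.
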(event `FallAlongSpline`
  (bind (_fail_tile_location_x _fail_tile_location_y _fail_tile_location_z) (`KismetMathLibrary.BreakVector` (`self.Fail Tile Location`)))
  (bind _enemyspline (`self.EnemySpline`))
  (bind (_fail_tile_location_x_2 _fail_tile_location_y_2 _fail_tile_location_z_2) (`KismetMathLibrary.BreakVector` (`self.Fail Tile Location`)))
  (bind _spline (`/Game/bp/BP_Spline.Spline` (`self.EnemySpline`)))
  (bind _spline_2 (`/Game/bp/BP_Spline.Spline` _enemyspline))
  ;[1 1 1] FallAlongSpline
  (`self.K2_SetActorLocation` _enemyspline (`self.K2_GetActorLocation` self) false false)
  (`SplineComponent.SetLocationAtSplinePoint` _spline_2 1 (`KismetMathLibrary.MakeVector` _fail_tile_location_x (- _fail_tile_location_y 1.0) (+ _fail_tile_location_z 40.0)) "World" true)
  (`SplineComponent.SetLocationAtSplinePoint` _spline_2 2 (`KismetMathLibrary.MakeVector` _fail_tile_location_x_2 (- _fail_tile_location_y_2 1.0) (- _fail_tile_location_z_2 100.0)) "World" true)
  (bind (_direction _0to1) (`Timeline|Timeline_1` :!via `PlayFromStart`)
    (:`Update`
      (`self.K2_SetActorLocation` (`SplineComponent.GetLocationAtDistanceAlongSpline` _spline (`KismetMathLibrary.Lerp` 0.0 (`SplineComponent.GetSplineLength` _spline) _0to1) "World")))
    (:`Finished`
      ;[1 1 1] Destroy Actors
      (`self.K2_DestroyActor` (`self.EnemySpline`))
      (`self.K2_DestroyActor`))))

(event `SpawnAndMoveSpline`
  (bind _enemyspline (`self.EnemySpline`))
  (bind (_returnvalue_x _returnvalue_y _returnvalue_z) (`KismetMathLibrary.BreakVector` (`self.K2_GetActorLocation` (`self.CurrentTile`))))
  (bind (_returnvalue_x_2 _returnvalue_y_2 _returnvalue_z_2) (`KismetMathLibrary.BreakVector` (`self.K2_GetActorLocation` (`self.currentTile`))))
  (bind _spline (`/Game/bp/BP_Spline.Spline` (`self.EnemySpline`)))
  (bind _spline_2 (`/Game/bp/BP_Spline.Spline` _enemyspline))
  ;[1 1 1] Spawn Spline
  (`self.K2_SetActorLocation` _enemyspline (`self.K2_GetActorLocation` self) false false)
  (`SplineComponent.SetLocationAtSplinePoint` _spline_2 1 (`KismetMathLibrary.MakeVector` _returnvalue_x (+ _returnvalue_y 0.2) (+ _returnvalue_z 40.0)) "World" true)
  (`SplineComponent.SetLocationAtSplinePoint` _spline_2 2 (`KismetMathLibrary.MakeVector` _returnvalue_x_2 (+ _returnvalue_y_2 0.2) (+ _returnvalue_z_2 10.0)) "World" true)
  (bind (_direction _0to1) (`Timeline|Timeline_0` :!via `PlayFromStart`)
    (:`Update`
      (`self.K2_SetActorLocation` (`SplineComponent.GetLocationAtDistanceAlongSpline` _spline (`KismetMathLibrary.Lerp` 0.0 (`SplineComponent.GetSplineLength` _spline) _0to1) "World")))
    (:`Finished`
      ;[1 1 1] Let Balls Start to Move
      (set `self.Activate` true))))

(event `self.ReceiveBeginPlay`
  ;[1 1 1] Begin Play
  ;[1 1 1] Create Spline and Move
  (`self.InitSpline`)
  (`self.SpawnAndMoveSpline`))

(fn `InitSpline`
  (bind _returnvalue (`|SpawnActorFromClass` "/Game/bp/BP_Spline.BP_Spline_C" (`self.GetTransform` self) "Undefined" "OverrideRootScale" null null))
  (set `self.EnemySpline` _returnvalue))

(fn `UserConstructionScript`)