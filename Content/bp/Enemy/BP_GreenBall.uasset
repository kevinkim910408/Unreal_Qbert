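; Green ball enemy that hops downward across linked tiles until it drops off the edge.
; Once activated, a looping two-second timer randomly picks the current tile's down-left or down-right neighbor.
; It reshapes a separate spline actor toward that tile, and a timeline moves the ball along it.
; With no tile on the chosen side, it sets an off-edge fail location, calls FallAlongSpline and stops the timer.
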(event `self.ReceiveBeginPlay`
  (`parent.ReceiveBeginPlay`))

(event `self.ReceiveTick`
  (params (DeltaSeconds :type "Float (single-precision)"))
  (if (`self.Activate`)
    ;[1 1 1] 이동한다 초록볼이
    (`/Engine/EditorBlueprintResources/StandardMacros.DoOnce` false
      (:`Completed`
        (bind _returnvalue (`KismetSystemLibrary.K2_SetTimer` null "NewSpline_RedBall" (`KismetMathLibrary.RandomFloatInRange` 2.0 2.0) true))
        (set `self.GreenBallMovement` _returnvalue)))))

(event `NewSpline_RedBall`
  (bind _currenttile (`self.CurrentTile`))
  (bind _enemyspline (`self.EnemySpline`))
  (bind _currenttile_2 (`self.CurrentTile`))
  (bind (_returnvalue_x _returnvalue_y _returnvalue_z) (`KismetMathLibrary.BreakVector` (`self.K2_GetActorLocation` (`self.CurrentTile`))))
  (bind (_returnvalue_x_2 _returnvalue_y_2 _returnvalue_z_2) (`KismetMathLibrary.BreakVector` (`self.K2_GetActorLocation` (`self.currentTile`))))
  (bind _spline (`/Game/bp/BP_Spline.Spline` (`self.EnemySpline`)))
  (bind _spline_2 (`/Game/bp/BP_Spline.Spline` _enemyspline))
  (bind _downlefttile (`/Game/bp/BP_Tile.DownLeftTile` _currenttile))
  (bind _downrighttile (`/Game/bp/BP_Tile.DownRightTile` _currenttile_2))
  (if (== (`KismetMathLibrary.RandomIntegerInRange` 0 1) 1)
    ;[1 1 1] Down Left
    (`/Engine/EditorBlueprintResources/StandardMacros.IsValid` _downlefttile
      (:`Is Valid`
        (set `self.CurrentTile` _downlefttile)
        ;[1 1 1] Set Spline for the balls
        (`self.K2_SetActorLocation` _enemyspline (`self.K2_GetActorLocation` self) false false :!label _label)
        (`SplineComponent.SetLocationAtSplinePoint` _spline_2 1 (`KismetMathLibrary.MakeVector` _returnvalue_x (+ _returnvalue_y 0.2) (+ _returnvalue_z 40.0)) "World" true)
        (`SplineComponent.SetLocationAtSplinePoint` _spline_2 2 (`KismetMathLibrary.MakeVector` _returnvalue_x_2 (+ _returnvalue_y_2 0.2) (+ _returnvalue_z_2 13.0)) "World" true)
        ;[1 1 1] Follow Spline to move
        (bind (_direction _0to1) (`Timeline|Timeline_1_0` :!via `PlayFromStart`)
          (:`Update`
            (`self.K2_SetActorLocation` (`SplineComponent.GetLocationAtDistanceAlongSpline` _spline (`KismetMathLibrary.Lerp` 0.0 (`SplineComponent.GetSplineLength` _spline) _0to1) "World")))))
      (:`Is Not Valid`
        ;[1 1 1] If Balls Drop from the tile
        (set `self.Fail Tile Location` (+ (`self.K2_GetActorLocation` _currenttile) (-16.0 0.0 -24.0)))
        (`self.FallAlongSpline`)
        (`KismetSystemLibrary.K2_ClearAndInvalidateTimerHandle` (`self.GreenBallMovement`))))
    (else
      ;[1 1 1] Down Right
      (`/Engine/EditorBlueprintResources/StandardMacros.IsValid` _downrighttile
        (:`Is Valid`
          (set `self.CurrentTile` _downrighttile)
          (goto _label))
        (:`Is Not Valid`
          ;[1 1 1] If Balls Drop from the tile
          (set `self.Fail Tile Location` (+ (`self.K2_GetActorLocation` _currenttile_2) (16.0 0.0 -24.0)))
          (`self.FallAlongSpline`)
          (`KismetSystemLibrary.K2_ClearAndInvalidateTimerHandle` (`self.GreenBallMovement`)))))))

(fn `UserConstructionScript`)