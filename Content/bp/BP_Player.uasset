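; Q*bert-style player that hops diagonally between linked tiles, rides elevators and falls off edges.
; Four input actions pick the CurrentTile's neighbour, ignoring presses mid-move, and set sound and facing sprite.
; Timelines move the player along a spawned BP_Spline, reshaped per move: landings recolour the tile, elevators carry the player to the first tile.
; A missing neighbour triggers a fall that costs a life and respawns the player on that first tile.
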(event `MoveAlongSpline`
  (bind (_returnvalue_x _returnvalue_y _returnvalue_z) (`KismetMathLibrary.BreakVector` (`self.K2_GetActorLocation` (`self.currentTile`))))
  (bind (_returnvalue_x_2 _returnvalue_y_2 _returnvalue_z_2) (`KismetMathLibrary.BreakVector` (`self.K2_GetActorLocation` (`self.currentTile`))))
  (bind _spline (`/Game/bp/BP_Spline.Spline` (`self.QbertSpline`)))
  (bind _spline_2 (`/Game/bp/BP_Spline.Spline` (`self.QbertSpline`)))
  ;[1 1 1] MoveAlongSpline
  (`self.K2_SetActorLocation` (`self.QbertSpline`) (`self.K2_GetActorLocation` self) false false)
  (`SplineComponent.SetLocationAtSplinePoint` _spline 1 (`KismetMathLibrary.MakeVector` _returnvalue_x (+ _returnvalue_y 0.2) (+ _returnvalue_z 40.0)) "World" true)
  (`SplineComponent.SetLocationAtSplinePoint` _spline 2 (`KismetMathLibrary.MakeVector` _returnvalue_x_2 (+ _returnvalue_y_2 0.2) (+ _returnvalue_z_2 16.0)) "World" true)
  (bind (_direction _0to1) (`Timeline|타임라인_0` :!via `PlayFromStart`)
    (:`Update`
      (`self.K2_SetActorLocation` (`SplineComponent.GetLocationAtDistanceAlongSpline` _spline_2 (`KismetMathLibrary.Lerp` 0.0 (`SplineComponent.GetSplineLength` _spline_2) _0to1) "World")))
    (:`Finished`
      (if (`self.isElevator`)
        (`self.ElevatorAlongSpline`)
        (else
          (set `self.isPlayerMoving` false)
          (`self.ChangeTile`))))))

(event `ChangeTile`
  ;[1 1 1] Change Tile
  (`/Game/bp/BP_Tile.changeColor` (`self.currentTile`)))

(event `ElevatorAlongSpline`
  (bind _elevatortemp (`self.ElevatorTemp`))
  (bind _spline (`/Game/bp/BP_Spline.Spline` (`self.QbertSpline`)))
  (bind _spline_2 (`/Game/bp/BP_Spline.Spline` (`self.QbertSpline`)))
  (bind _spline_3 (`/Game/bp/BP_Spline.Spline` (`self.QbertSpline`)))
  (bind _spline_4 (`/Game/bp/BP_Spline.Spline` (`self.QbertSpline`)))
  (`self.K2_SetActorLocation` (`self.QbertSpline`) (`self.K2_GetActorLocation`) false false)
  (`|ExecutionSequence`
    (:`then_0`
      (`SplineComponent.SetSplinePointType` _spline_4 0 "Linear" true))
    (:`then_1`
      (`SplineComponent.SetSplinePointType` _spline_4 1 "Linear" true)
      (set `self.ArcSplineSecondPointOffset` (0.0 0.3 40.0))
      (`SplineComponent.SetLocationAtSplinePoint` _spline_2 1 (+ (`self.K2_GetActorLocation` (`|GetArrayItem` (`/Game/bp/BP_MyMode.Array of Tiles` (cast `/Game/bp/BP_MyMode` (`GameplayStatics.GetGameMode`) :!pure true)))) (`self.ArcSplineSecondPointOffset`)) "World" false)
      (set `self.ArcSplineSecondPointOffset` (0.0 0.3 16.0))
      (`SplineComponent.SetLocationAtSplinePoint` _spline_2 2 (+ (`self.K2_GetActorLocation` (`|GetArrayItem` (`/Game/bp/BP_MyMode.Array of Tiles` (cast `/Game/bp/BP_MyMode` (`GameplayStatics.GetGameMode`) :!pure true)))) (`self.ArcSplineSecondPointOffset`)) "World" true)
      (bind (_direction _0_to_1) (`Timeline|Timeline_1` :!via `PlayFromStart`)
        (:`Update`
          (bind _returnvalue (`SplineComponent.GetLocationAtDistanceAlongSpline` _spline_3 (`KismetMathLibrary.Lerp` 0.0 (`SplineComponent.GetSplineLength` _spline_3) _0_to_1) "World"))
          (`self.K2_SetActorLocation` _returnvalue)
          (`/Engine/EditorBlueprintResources/StandardMacros.IsValid` _elevatortemp
            (:`Is Valid`
              (`self.K2_SetActorLocation` _elevatortemp (+ _returnvalue (0.0 -0.2 -8.0)) false false)
              (if (== (`self.K2_GetActorLocation`) (`SplineComponent.GetLocationAtSplinePoint` (`/Game/bp/BP_Spline.Spline` (`self.QbertSpline`)) 1 "World") :`ErrorTolerance` 5.0)
                (`self.K2_DestroyActor` (`self.ElevatorTemp`))
                (set `self.ElevatorTemp` null)))))
        (:`Finished`
          (`|ExecutionSequence`
            (:`then_0`
              (`SplineComponent.SetSplinePointType` _spline 0 "Curve" true))
            (:`then_1`
              (`SplineComponent.SetSplinePointType` _spline 1 "Curve" true)
              (set `self.isPlayerMoving` false)
              (set `self.isElevator` false)
              (set `self.currentTile` (`|GetArrayItem` (`/Game/bp/BP_MyMode.Array of Tiles` (cast `/Game/bp/BP_MyMode` (`GameplayStatics.GetGameMode`) :!pure true)))))))))))

(event `FallAlongSpline`
  (bind (_falltilelocation_x _falltilelocation_y _falltilelocation_z) (`KismetMathLibrary.BreakVector` (`self.FallTileLocation`)))
  (bind (_falltilelocation_x_2 _falltilelocation_y_2 _falltilelocation_z_2) (`KismetMathLibrary.BreakVector` (`self.FallTileLocation`)))
  (bind _spline (`/Game/bp/BP_Spline.Spline` (`self.QbertSpline`)))
  (bind _spline_2 (`/Game/bp/BP_Spline.Spline` (`self.QbertSpline`)))
  ;[1 1 1] FallAlongSpline
  (`self.K2_SetActorLocation` (`self.QbertSpline`) (`self.K2_GetActorLocation` self) false false)
  (`SplineComponent.SetLocationAtSplinePoint` _spline_2 1 (`KismetMathLibrary.MakeVector` _falltilelocation_x_2 (- _falltilelocation_y_2 1.0) (+ _falltilelocation_z_2 40.0)) "World" true)
  (`SplineComponent.SetLocationAtSplinePoint` _spline_2 2 (`KismetMathLibrary.MakeVector` _falltilelocation_x (- _falltilelocation_y 1.0) (- _falltilelocation_z 100.0)) "World" true)
  (bind (_direction _0to1) (`Timeline|Timeline_0` :!via `PlayFromStart`)
    (:`Update`
      (`self.K2_SetActorLocation` (`SplineComponent.GetLocationAtDistanceAlongSpline` _spline (`KismetMathLibrary.Lerp` 0.0 (`SplineComponent.GetSplineLength` _spline) _0to1) "World")))
    (:`Finished`
      ;[1 1 1] Reset Character Position/ Life - 1
      (bind _result (`/Engine/EditorBlueprintResources/StandardMacros.DecrementInt` (`self.PlayerLife`))
        (:`  `
          (`KismetSystemLibrary.PrintString` (`KismetStringLibrary.Conv_IntToString` _result))
          (bind _asbp_my_mode (cast `/Game/bp/BP_MyMode` (`GameplayStatics.GetGameMode`)))
          (bind _output (`|GetArrayItem` (`/Game/bp/BP_MyMode.Array of Tiles` _asbp_my_mode)))
          (`self.K2_SetActorLocation` (+ (`self.K2_GetActorLocation` _output) (0.0 0.2 16.0)))
          (set `self.isPlayerMoving` false)
          (set `self.currentTile` _output))))))

(event `InputAction|MoveLeftUp_7`
  (params (Key :type "Key Structure"))
  (bind _currenttile (`self.currentTile`))
  (bind _uplefttile (`/Game/bp/BP_Tile.UpLeftTile` _currenttile))
  (bind (_asbp_elevator _bsuccess) (cast `/Game/bp/BP_Elevator` _uplefttile :!pure true))
  (:`Pressed`
    (if (not (`self.isPlayerMoving`))
      (`/Engine/EditorBlueprintResources/StandardMacros.IsValid` _uplefttile
        (:`Is Valid`
          (if _bsuccess
            ;[1 1 1] Elevator
            (set `self.isElevator` true)
            (set `self.ElevatorTemp` _asbp_elevator)
            (set `self.isPlayerMoving` true)
            (set `self.currentTile` _asbp_elevator)
            (`self.MoveAlongSpline`)
            (`GameplayStatics.PlaySound2D` "/Game/Sounds/Elevator.Elevator" 1.0 1.0 0.0 null null)
            (else
              ;[1 1 1] Tile
              (set `self.isPlayerMoving` true)
              (set `self.currentTile` _uplefttile)
              (`self.MoveAlongSpline`)
              (`GameplayStatics.PlaySound2D` "/Game/Sounds/Jump.Jump" 1.0 1.0 0.0 null null))))
        (:`Is Not Valid`
          (set `self.FallTileLocation` (+ (`self.K2_GetActorLocation` _currenttile) (-16.0 0.0 24.0)))
          (set `self.isPlayerMoving` true)
          (`self.FallAlongSpline`)
          (`GameplayStatics.PlaySound2D` "/Game/Sounds/QbertDropped.QbertDropped" 1.0 1.0 0.0 null null)))
      (`PaperSpriteComponent.SetSprite` (`self.PaperSprite`) "/Game/Sprite/Player/Player07.Player07" :!label _label))))

(event `InputAction|MoveRighttUp_9`
  (params (Key :type "Key Structure"))
  (bind _currenttile (`self.currentTile`))
  (bind _uprighttile (`/Game/bp/BP_Tile.UpRightTile` _currenttile))
  (bind (_asbp_elevator _bsuccess) (cast `/Game/bp/BP_Elevator` _uprighttile :!pure true))
  (:`Pressed`
    (if (not (`self.isPlayerMoving`))
      (`/Engine/EditorBlueprintResources/StandardMacros.IsValid` _uprighttile
        (:`Is Valid`
          (if _bsuccess
            ;[1 1 1] Elevator
            (set `self.isElevator` true)
            (set `self.ElevatorTemp` _asbp_elevator)
            (set `self.isPlayerMoving` true)
            (set `self.currentTile` _asbp_elevator)
            (`self.MoveAlongSpline`)
            (`GameplayStatics.PlaySound2D` "/Game/Sounds/Elevator.Elevator" 1.0 1.0 0.0 null null)
            (else
              ;[1 1 1] Tile
              (set `self.isPlayerMoving` true)
              (set `self.currentTile` _uprighttile)
              (`self.MoveAlongSpline`)
              (`GameplayStatics.PlaySound2D` "/Game/Sounds/Jump.Jump" 1.0 1.0 0.0 null null))))
        (:`Is Not Valid`
          (set `self.FallTileLocation` (+ (`self.K2_GetActorLocation` _currenttile) (16.0 0.0 24.0)))
          (set `self.isPlayerMoving` true)
          (`self.FallAlongSpline`)
          (`GameplayStatics.PlaySound2D` "/Game/Sounds/QbertDropped.QbertDropped" 1.0 1.0 0.0 null null)))
      (`PaperSpriteComponent.SetSprite` (`self.PaperSprite`) "/Game/Sprite/Player/Player06.Player06" :!label _label_2))))

(event `InputAction|MoveLeftDown_1`
  (params (Key :type "Key Structure"))
  (bind _currenttile (`self.currentTile`))
  (bind _downlefttile (`/Game/bp/BP_Tile.DownLeftTile` _currenttile))
  (:`Pressed`
    (if (not (`self.isPlayerMoving`))
      (`/Engine/EditorBlueprintResources/StandardMacros.IsValid` _downlefttile
        (:`Is Valid`
          (set `self.isPlayerMoving` true)
          (set `self.currentTile` _downlefttile)
          (`self.MoveAlongSpline`)
          (`GameplayStatics.PlaySound2D` "/Game/Sounds/Jump.Jump" 1.0 1.0 0.0 null null)
          (goto _label))
        (:`Is Not Valid`
          (set `self.FallTileLocation` (+ (`self.K2_GetActorLocation` _currenttile) (-16.0 0.0 -24.0)))
          (set `self.isPlayerMoving` true)
          (`self.FallAlongSpline`)
          (`GameplayStatics.PlaySound2D` "/Game/Sounds/QbertDropped.QbertDropped" 1.0 1.0 0.0 null null)
          (goto _label))))))

(event `InputAction|MoveRightDown_3`
  (params (Key :type "Key Structure"))
  (bind _currenttile (`self.currentTile`))
  (bind _downrighttile (`/Game/bp/BP_Tile.DownRightTile` _currenttile))
  (:`Pressed`
    (if (not (`self.isPlayerMoving`))
      (`/Engine/EditorBlueprintResources/StandardMacros.IsValid` _downrighttile
        (:`Is Valid`
          (set `self.isPlayerMoving` true)
          (set `self.currentTile` _downrighttile)
          (`self.MoveAlongSpline`)
          (`GameplayStatics.PlaySound2D` "/Game/Sounds/Jump.Jump" 1.0 1.0 0.0 null null)
          (goto _label_2))
        (:`Is Not Valid`
          (set `self.FallTileLocation` (+ (`self.K2_GetActorLocation` _currenttile) (16.0 0.0 -24.0)))
          (set `self.isPlayerMoving` true)
          (`self.FallAlongSpline`)
          (`GameplayStatics.PlaySound2D` "/Game/Sounds/QbertDropped.QbertDropped" 1.0 1.0 0.0 null null)
          (goto _label_2))))))

(fn `InitQbert`
  (bind _returnvalue (`|SpawnActorFromClass` "/Game/bp/BP_Spline.BP_Spline_C" (`self.GetTransform` self) "Undefined" "OverrideRootScale" null null))
  (set `self.QbertSpline` _returnvalue)
  (bind _asbp_my_mode (cast `/Game/bp/BP_MyMode` (`GameplayStatics.GetGameMode`)))
  (set `self.currentTile` (`|GetArrayItem` (`/Game/bp/BP_MyMode.Array of Tiles` _asbp_my_mode))))

(fn `UserConstructionScript`)