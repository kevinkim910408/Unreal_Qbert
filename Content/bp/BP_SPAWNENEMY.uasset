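; BP_SPAWNENEMY is a spawner that places a red ball enemy on the tile board.
; BeginPlay sets a non-looping one-second timer that calls SpawnRedBall by function name.
; SpawnRedBall spawns BP_REDBALL above a random tile, index 1 or 2, from BP_MyMode's ArrayOfTiles, and supplies its CurrentTile.
; A longer randomized timer for SpawnRedBall is left unconnected, so spawning does not repeat.
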(event `SpawnRedBall`
  (bind _output (`|GetArrayItem` (`/Game/bp/BP_MyMode.Array of Tiles` (cast `/Game/bp/BP_MyMode` (`GameplayStatics.GetGameMode`) :!pure true)) (`KismetMathLibrary.RandomIntegerInRange` 1 2)))
  (`|SpawnActorFromClass` "/Game/bp/BP_REDBALL.BP_REDBALL_C" (`KismetMathLibrary.MakeTransform` (+ (`self.K2_GetActorLocation` _output) (0.0 0.2 150.0))) "Undefined" "OverrideRootScale" null _output null))

(event `self.ReceiveBeginPlay`
  (`KismetSystemLibrary.K2_SetTimer` null "SpawnRedBall" (`KismetMathLibrary.RandomFloatInRange` 1.0 1.0)))

(fn `UserConstructionScript`)