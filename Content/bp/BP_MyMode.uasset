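; Game mode for a Q*bert-style game that builds the tile pyramid and keeps the score.
; BeginPlay spawns triangular rows of BP_Tile into an array, links them, then creates the HUD, initializes the player and spawns BP_SPAWNENEMY.
; ConnectTiles walks the flat array using row counters to set each tile's four diagonal neighbors, hooking elevators into both outer edges of the fifth row.
; ScoreIncrease adds a fixed amount to the score.
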(event `self.ReceiveBeginPlay`
  (`|ExecutionSequence`
    (:`then_0`
      ;[1 1 1] Tile make
      (for _index (range (`self.FloorLevel`))
        (for _index_2 (range (+ _index 1))
          (bind _returnvalue (`|SpawnActorFromClass` "/Game/bp/BP_Tile.BP_Tile_C" (`KismetMathLibrary.MakeTransform` (`KismetMathLibrary.MakeVector` (+ (* _index_2 32.0) (* _index -16.0)) 5.0 (* _index -24.0))) "Undefined" "OverrideRootScale" null null))
          (`KismetArrayLibrary.Array_Add` (`self.Array of Tiles`) _returnvalue))))
    (:`then_1`
      (`self.ConnectTiles`)
      (bind _returnvalue_2 (`|CreateWidget` "/Game/bp/WBP/WBP_HUD.WBP_HUD_C"))
      (`UserWidget.AddToViewport` _returnvalue_2 0)
      (bind _asbp_player (cast `/Game/bp/BP_Player` (`GameplayStatics.GetPlayerPawn` 0)))
      (`/Game/bp/BP_Player.InitQbert` _asbp_player))
    (:`then_2`
      (`|SpawnActorFromClass` "/Game/bp/BP_SPAWNENEMY.BP_SPAWNENEMY_C" (`KismetMathLibrary.MakeTransform` (0.0 0.0 0.0)) "Undefined" "OverrideRootScale" null null))))

(fn `ConnectTiles`
  (locals (FloorCount :type Integer :default 1) (FirstIndex :type Integer) (LasIndex :type Integer))
  ;[1 1 1] Construct
  (for (_array_element _array_index) (`self.Array of Tiles`)
    (`|ExecutionSequence`
      (:`then_0`
        ;[1 1 1] If Current level == Max level
        (if (not (== (`local.FloorCount`) (`self.FloorLevel`)))
          (`|ExecutionSequence`
            (:`then_0`
              ;[1 1 1] Left Down
              (set `/Game/bp/BP_Tile.DownLeftTile` (`|GetArrayItem` (`self.Array of Tiles`) (+ _array_index (`local.FloorCount`))) _array_element))
            (:`then_1`
              ;[1 1 1] Right Down
              (set `/Game/bp/BP_Tile.DownRightTile` (`|GetArrayItem` (`self.Array of Tiles`) (+ _array_index (+ (`local.FloorCount`) 1))) _array_element)))))
      (:`then_1`
        (if (not (== (`local.FloorCount`) 1))
          (`|ExecutionSequence`
            (:`then_0`
              (if (not (== (`local.FirstIndex`) _array_index))
                ;[1 1 1] Left Up
                (set `/Game/bp/BP_Tile.UpLeftTile` (`|GetArrayItem` (`self.Array of Tiles`) (- _array_index (`local.FloorCount`))) _array_element)))
            (:`then_1`
              (if (not (== _array_index (`local.LasIndex`)))
                ;[1 1 1] Right Up
                (set `/Game/bp/BP_Tile.UpRightTile` (`|GetArrayItem` (`self.Array of Tiles`) (- _array_index (- (`local.FloorCount`) 1))) _array_element))))))
      (:`then_2`
        ;[1 1 1] Elevator
        (if (== (`local.FloorCount`) 5)
          (`|ExecutionSequence`
            (:`then_0`
              (if (== (`local.FirstIndex`) _array_index)
                (bind _output (`|GetArrayItem` (`self.Array of Tiles`) _array_index))
                (bind _returnvalue (`|SpawnActorFromClass` "/Game/bp/BP_Elevator.BP_Elevator_C" (`KismetMathLibrary.MakeTransform` (+ (`self.K2_GetActorLocation` _output) (-16.0 0.0 24.0))) "Undefined" "OverrideRootScale" null null))
                (set `/Game/bp/BP_Tile.UpLeftTile` _returnvalue _output)))
            (:`then_1`
              (if (== (`local.LasIndex`) _array_index)
                (bind _output_2 (`|GetArrayItem` (`self.Array of Tiles`) _array_index))
                (bind _returnvalue_2 (`|SpawnActorFromClass` "/Game/bp/BP_Elevator.BP_Elevator_C" (`KismetMathLibrary.MakeTransform` (+ (`self.K2_GetActorLocation` _output_2) (16.0 0.0 24.0))) "Undefined" "OverrideRootScale" null null))
                (set `/Game/bp/BP_Tile.UpRightTile` _returnvalue_2 _output_2))))))
      (:`then_3`
        ;[1 1 1] Level ++
        (if (== _array_index (`local.LasIndex`))
          (`/Engine/EditorBlueprintResources/StandardMacros.IncrementInt` (`local.FloorCount`)
            (:`  `
              (`|ExecutionSequence`
                (:`then_0`
                  (set `local.FirstIndex` (+ (`local.LasIndex`) 1)))
                (:`then_1`
                  (set `local.LasIndex` (+ (`local.FloorCount`) (`local.LasIndex`))))))))))))

(fn `ScoreIncrease`
  (set `self.CurrentScore` (+ (`self.CurrentScore`) 25)))

(fn `UserConstructionScript`)